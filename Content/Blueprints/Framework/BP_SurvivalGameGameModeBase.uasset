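; Survival game mode base that overrides player start selection to spawn players at BP_SurvivalPlayerStart actors.
; BeginPlay caches every such actor in PlayerStarts, and FindPlayerStart picks one at random, marks it used and returns it.
; When the pick is already used, a while loop clears it to None instead of re-rolling.
; An author note flags spawn point retrieval as faulty.
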(event EventBeginPlay
  (bind _outactors (Actor|GetAllActorsOfClass "/Game/Blueprints/BP_SurvivalPlayerStart.BP_SurvivalPlayerStart_C"))
  (Variables|Default|SetPlayerStarts _outactors))

(event EventTick
  (params (DeltaSeconds :type Float%20%28single-precision%29)))

(fn ConstructionScript)

(fn FindPlayerStart
  (params (Player :type Controller%20Object%20Reference) (IncomingName :type String))
  (bind _playerstarts (Variables|Default|GetPlayerStarts))
  ;[1 1 1] something wrong with geting spawn point
  (LocalVariables|SetPlayerStart (Utilities|Array|Get(acopy) _playerstarts (Math|Random|RandomIntegerinRange 0 (- (Utilities|Array|Length _playerstarts) 1))))
  (while (Variables|/Game/Blueprints/BP_SurvivalPlayerStart.BP_SurvivalPlayerStart_C|GetUsed (LocalVariables|GetPlayerStart))
    (LocalVariables|SetPlayerStart 0))
  (Default|MarkUsed (LocalVariables|GetPlayerStart))
  (return (LocalVariables|GetPlayerStart)))